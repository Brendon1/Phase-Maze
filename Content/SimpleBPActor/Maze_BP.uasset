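; Maze_BP is a maze board actor that the player tilts with input axes.
; The TiltLeft and TiltRight axis events both add world roll to Boardmesh, scaled by RotationSpeed.
; A node chain that would clamp roll to a narrow range is never executed, so this graph does not limit the tilt.
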(event Input|AxisEvents|InputAxisTiltLeft
  (params (AxisValue :type Float%20%28single-precision%29))
  (Transformation|AddWorldRotation (Variables|Default|GetBoardmesh) (Math|Rotator|MakeRotator (* AxisValue (Variables|Default|GetRotationSpeed)) 0.0 0.0) false false))

(event Input|AxisEvents|InputAxisTiltRight
  (params (AxisValue :type Float%20%28single-precision%29))
  (Transformation|AddWorldRotation (Variables|Default|GetBoardmesh) (Math|Rotator|MakeRotator (* AxisValue (Variables|Default|GetRotationSpeed)) 0.0 0.0) false false))

(fn ConstructionScript)